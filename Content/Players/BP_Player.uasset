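; Player character for a multiplayer bumping game, steered by stick direction and propelled by charge-and-release dashes.
; A timeline fills the charge gauge while held; release converts it into speed, applied as decaying world offsets in Tick.
; Box overlaps between players trade movement through mutual CrashEvent calls, guarded by IsMoveUpdate, with smash effect and controller rumble.
; Helper functions spawn state particles and set one of four machine mesh and color variants.
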(event `self.ReceiveTick`
  (params (DeltaSeconds :type "Float (single-precision)"))
  (bind _inputaxis (`self.inputAxis`))
  (bind _returnvalue (`KismetMathLibrary.MakeVector2D` (`self.axis_X`) (`self.axis_Y`)))
  (bind (_returnvalue_x _returnvalue_y) (`KismetMathLibrary.BreakVector2D` (* (`self.move`) (`self.speed`))))
  (bind _returnvalue_2 (- (`self.speed`) 5.0))
  (bind _degree (`self.dot` (0.0 1.0) _inputaxis))
  (bind _sign (`self.cross` (0.0 1.0) _inputaxis))
  (`|ExecutionSequence`
    (:`then_0`
      ;[1 1 1] 入力方向更新
      (if (>= (`KismetMathLibrary.VSize2D` _returnvalue) 0.8)
        (set `self.inputAxis` (`KismetMathLibrary.Normal2D` _returnvalue))
        ;[1 1 1] 入力値方向に向く
        (if (== _sign 0.0)
          (bind _output_get (set `self.rotation` (`KismetMathLibrary.MakeRotator` 0.0 0.0 _degree)))
          (`self.K2_SetActorRotation` _output_get)
          (else
            (bind _output_get_2 (set `self.rotation` (`KismetMathLibrary.MakeRotator` 0.0 0.0 (* _sign _degree))))
            (`self.K2_SetActorRotation` _output_get_2)))
        (else
          (set `self.inputAxis` (0.0 0.0)))))
    (:`then_1`
      ;[1 1 1] ダッシュ
      (`self.K2_AddActorWorldOffset` (`KismetMathLibrary.MakeVector` _returnvalue_y _returnvalue_x))
      (if (<= _returnvalue_2 0.0)
        (set `self.speed` 0.0)
        (else
          (set `self.speed` _returnvalue_2)
          (`self.EffectCreater` "NewEnumerator0"))))))

(event `InputAxis|AxisX`
  (params (AxisValue :type "Float (single-precision)"))
  (set `self.axis_X` AxisValue))

(event `InputAxis|AxisY`
  (params (AxisValue :type "Float (single-precision)"))
  (set `self.axis_Y` AxisValue))

(event `self.ReceiveBeginPlay`)

(event `InputAction|Charge`
  (params (Key :type "Key Structure"))
  ;[1 1 1] チャージ処理
  (:`Pressed`
    (`self.ChargeStart`))
  (:`Released`
    (`self.ChargeEnd`)))

(event `ChargeStart`
  ;[1 1 1] チャージ処理
  (`Timeline|ChargeTimer` :!via `PlayFromStart` :!label _label
    (:`Update`
      (if (<= (`self.ChargeGage`) 100.0)
        (`/Engine/EditorBlueprintResources/StandardMacros.IncrementFloat` (`self.ChargeGage`)
          (:`  `
            (`self.EffectCreater` "NewEnumerator1")))
        (else
          (`|ExecutionSequence`
            (:`then_0`
              (`/Engine/EditorBlueprintResources/StandardMacros.DoOnce` false :!label _label_2
                (:`Completed`
                  (`self.EffectCreater` "NewEnumerator2"))))
            (:`then_1`
              (`self.EffectCreater` "NewEnumerator3"))))))))

(event `ChargeEnd`
  ;[1 1 1] チャージ処理
  (`|ExecutionSequence`
    (:`then_0`
      (if (== (`self.inputAxis`) (0.0 0.0))
        (set `self.ChargeGage` 0.0)
        (goto _label :!via `Stop`)
        (else
          (set `self.move` (`self.inputAxis`))
          (set `self.speed` (* (`self.ChargeGage`) 2.0))
          (set `self.ChargeGage` 0.0)
          (goto _label :!via `Stop`))))
    (:`then_1`
      (goto _label_2 :!via `Reset`))))

(event `DeadEvent`
  (set `MovementComponent.Velocity` (0.0 0.0 0.0) (`self.CharacterMovement`))
  (`self.EffectCreater` "NewEnumerator5")
  (goto _label :!via `Stop`))

(event `CrashEnd`
  ;[1 1 1] ぶつかったときの処理
  (set `self.isMoveUpdate` false))

(event `CrashEvent`
  (params (move :type "Vector2D Structure") (speed :type "Float (double-precision)") (crashPlayer :type "/Game/Players/BP_Player Object Reference"))
  ;[1 1 1] ぶつかったときの処理
  (if (not (`self.isMoveUpdate`))
    (set `self.newMove` move)
    (set `self.newSpeed` speed)
    (set `self.isMoveUpdate` true)
    (`self.CrashEvent` crashPlayer (`self.move`) (`self.speed`) self)
    (`self.EffectCreater` "NewEnumerator4")
    (`PlayerController.ClientPlayForceFeedback` (`GameplayStatics.GetPlayerController` (`self.num`)) "/Game/Effect/testEffectController.testEffectController" false false "None")
    (set `self.move` (`self.newMove`))
    (set `self.speed` (`self.newSpeed`))))

(event `self.Box.OnComponentBeginOverlap`
  (params (OverlappedComponent :type "PrimitiveComponent Object Reference") (OtherActor :type "Actor Object Reference") (OtherComp :type "PrimitiveComponent Object Reference") (OtherBodyIndex :type Integer) (bFromSweep :type Boolean) (SweepResult :type "HitResult Structure (by ref)"))
  ;[1 1 1] ぶつかったときの処理
  (bind _asbp_player (cast `/Game/Players/BP_Player` OtherActor))
  (`self.CrashEvent` _asbp_player (`self.move`) (`self.speed`) self))

(event `self.Box.OnComponentEndOverlap`
  (params (OverlappedComponent :type "PrimitiveComponent Object Reference") (OtherActor :type "Actor Object Reference") (OtherComp :type "PrimitiveComponent Object Reference") (OtherBodyIndex :type Integer))
  ;[1 1 1] ぶつかったときの処理
  (bind _asbp_player (cast `/Game/Players/BP_Player` OtherActor))
  (`self.CrashEnd` _asbp_player))

(fn `Dash`
  (`PrimitiveComponent.AddImpulse` (`self.CapsuleComponent`) (* (`self.LeftDirection`) (* (`self.ChargeGage`) 10000.0)) "None" false))

(fn `EffectCreater`
  (params (SpawnEffect :type "/Game/Players/PlayerEffect Enum" :default "NewEnumerator0"))
  (switch `/Game/Players/PlayerEffect` SpawnEffect
    (:`NewEnumerator0`
      (`GameplayStatics.SpawnEmitterAtLocation` "/Game/Effect/Particle/P_KnockBack.P_KnockBack" (`self.K2_GetActorLocation` self)))
    (:`NewEnumerator1`
      (`GameplayStatics.SpawnEmitterAtLocation` "/Game/Effect/Particle/P_Charge.P_Charge" (`self.K2_GetActorLocation` self)))
    (:`NewEnumerator2`
      (`GameplayStatics.SpawnEmitterAtLocation` "/Game/Effect/Particle/P_ChargeMax.P_ChargeMax" (`self.K2_GetActorLocation` self)))
    (:`NewEnumerator3`
      (`GameplayStatics.SpawnEmitterAtLocation` "/Game/Effect/Particle/P_ChargeNow.P_ChargeNow" (`self.K2_GetActorLocation` self)))
    (:`NewEnumerator4`
      (`GameplayStatics.SpawnEmitterAtLocation` "/Game/Effect/Particle/P_Attack.P_Attack" (`self.K2_GetActorLocation` self)))
    (:`NewEnumerator5`
      (`GameplayStatics.SpawnEmitterAtLocation` "/Game/Effect/Particle/P_Destroy.P_Destroy" (`self.K2_GetActorLocation` self)))))

(fn `MachineChange`
  (params (number :type Integer))
  (bind _machine (`self.Machine`))
  (switch `int` number
    (:`0`
      (`StaticMeshComponent.SetStaticMesh` _machine "/Game/Players/Machine/Machine_0.Machine_0")
      (`SceneComponent.SetWorldScale3D` _machine (4.0 4.0 4.0))
      (`PrimitiveComponent.SetMaterial` _machine 0 "/Game/Players/Machine/M_Red.M_Red"))
    (:`1`
      (`StaticMeshComponent.SetStaticMesh` _machine "/Game/Players/Machine/Machine_1.Machine_1")
      (`SceneComponent.SetWorldScale3D` _machine (6.0 6.0 6.0))
      (`PrimitiveComponent.SetMaterial` _machine 0 "/Game/Players/Machine/M_Blue.M_Blue"))
    (:`2`
      (`StaticMeshComponent.SetStaticMesh` _machine "/Game/Players/Machine/Machine_2.Machine_2")
      (`SceneComponent.SetWorldScale3D` _machine (6.0 6.0 6.0))
      (`PrimitiveComponent.SetMaterial` _machine 0 "/Game/Players/Machine/M_Green.M_Green"))
    (:`3`
      (`StaticMeshComponent.SetStaticMesh` _machine "/Game/Players/Machine/Machine_3.Machine_3")
      (`SceneComponent.SetWorldScale3D` _machine (7.0 7.0 7.0))
      (`PrimitiveComponent.SetMaterial` _machine 0 "/Game/Players/Machine/M_Yellow.M_Yellow"))))

(fn `UserConstructionScript`)